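; Board cell that awards points to the player whose turn it is when its effect is applied.
; On construction it runs the parent script, caches the game mode and tints itself blue.
; ApplyEffect adds ScoreIncrement through the game mode, then prints a "+score" message that shows the player's new total rather than the increment.
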(event EventBeginPlay)

(event Collision|EventActorBeginOverlap
  (params (OtherActor :type Actor%20Object%20Reference)))

(event EventTick
  (params (DeltaSeconds :type Float%20%28single-precision%29)))

(fn ConstructionScript
  (|CallParentFunction)
  (CallFunction|ReferenceGameMode)
  (Class|Cell|ChangeColor "(R=0.052083,G=0.467743,B=1.000000,A=1.000000)"))

(fn ApplyEffect
  (bind _gmref (Variables|Default|GetGMRef))
  (bind _current_player_turn_index (Default|GetCurrentPlayerTurnIndex _gmref))
  (Default|AddScore _gmref (Variables|Default|GetScoreIncrement) _current_player_turn_index)
  (Development|PrintString (Utilities|String|Append "+ " (Utilities|String|ToString(Integer) (Default|GetScore _gmref _current_player_turn_index)) " score !") true true "(R=1.000000,G=0.156157,B=0.000000,A=1.000000)" 5.0))
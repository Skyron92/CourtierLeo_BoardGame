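; BP_MemoryCard is a clickable card tile in the Memory minigame.
; On BeginPlay it assigns its Card component as the Mesh before running the parent's BeginPlay.
; Clicking the Card debug-prints its grid coordinate and passes that X and Y to the MemoryManager to pick the tile.
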(event OnClicked(Card)
  (params (TouchedComponent :type Primitive%20Component%20Object%20Reference) (ButtonPressed :type Key%20Structure :default "None"))
  (bind (_x _y) (Class|MemoryCard|GetCoord))
  (Development|PrintString (Utilities|String|Append (Utilities|String|ToString(Integer) _x) " " (Utilities|String|ToString(Integer) _y)))
  (Class|MemoryManager|PickTilebyCoord (Variables|Default|GetMemoryManager) _x _y))

(event EventBeginPlay
  (Variables|Default|Setmesh (Variables|Default|GetCard))
  (|CallParentFunction))

(event Collision|EventActorBeginOverlap
  (params (OtherActor :type Actor%20Object%20Reference)))

(event EventTick
  (params (DeltaSeconds :type Float%20%28single-precision%29)))

(fn ConstructionScript)
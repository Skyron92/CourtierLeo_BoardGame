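; BP_MoveCell is a board cell that moves the pawn by its Movement amount when its effect is applied.
; ApplyEffect calls MovePawn on the game mode reference and prints a French debug message with the movement and the result.
; DefineColor returns green for positive Movement and red otherwise.
; The construction script runs the parent's version, then calls ReferenceGameMode.
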(event EventBeginPlay)

(event Collision|EventActorBeginOverlap
  (params (OtherActor :type Actor%20Object%20Reference)))

(event EventTick
  (params (DeltaSeconds :type Float%20%28single-precision%29)))

(fn ConstructionScript
  (|CallParentFunction)
  (CallFunction|ReferenceGameMode))

(fn ApplyEffect
  (bind _movement (Variables|Default|GetMovement))
  (bind _cell (Default|MovePawn (Variables|Default|GetGMRef) _movement))
  (Development|PrintString (Utilities|String|Append "Je bouge de " (Utilities|String|ToString(Integer) _movement) " et je vais en " (Utilities|String|ToString(Integer) _cell))))

(fn DefineColor
  (if (> (Variables|Default|GetMovement) 0)
    (return "(R=0.000000,G=1.000000,B=0.083333,A=1.000000)")
    (else
      (return "(R=1.000000,G=0.000000,B=0.000000,A=1.000000)"))))
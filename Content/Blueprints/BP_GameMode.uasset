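; Game mode for a turn-based dice board game that runs setup, pawn movement, turns and the win message.
; BeginPlay sets the camera, menu and dice; StartGame spawns colored pawns and the dice widget.
; Each roll plays in the widget, whose animation-end event moves the pawn, applies the cell's effect and passes the turn.
; Player positions and scores live in the Game Instance; occupied cells are skipped recursively.
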(event Custom|SpawnPawns
  ;[1 1 1] Spawn All Pawns
  (for _index (range 0 (- (Variables|Player|GetPlayersNumber) 1))
    (bind _returnvalue (Game|SpawnActorfromClass "/Game/Blueprints/BP_BoardPawn.BP_BoardPawn_C" (Math|Transform|MakeTransform (Transformation|GetActorLocation (Utilities|Array|Get(acopy) (Variables|/Script/BoardGame.Board|GetStartCells (Variables|GameManagement|GetBoard)) _index)) (Variables|/Script/BoardGame.Cell|Getrotator (Utilities|Array|Get(acopy) (Variables|/Script/BoardGame.Board|GetStartCells (Variables|GameManagement|GetBoard)) _index)) "1.000000,1.000000,1.000000") "Undefined" "MultiplyWithRoot" 0 0))
    (bind _returnvalue_2 (Utilities|Array|AddUnique (Variables|Player|GetPawnsList) _returnvalue))
    ;[1 1 1] Color
    (bind _returnvalue_3 (Utilities|GetDataTableRow "/Game/DataTable/DT_PawnColor.DT_PawnColor" (.Value (Utilities|Map|Find (Variables|Player|GetPawnNameByID) _returnvalue_2)))
      (:then
        (Class|BoardPawn|SetColor _returnvalue (.color _returnvalue_3))))))

(event Custom|PlayerWin
  (Variables|Default|SetGameIsEnded true)
  (GameManagement|ModifyText (Utilities|Text|ToText(String) (Utilities|String|Append "Player " (Utilities|String|ToString(Integer) (Variables|Player|GetCurrentPlayerTurn)) " won !")))
  (Default|SetButtonState (Variables|UI|GetDiceWidget) false))

(event Custom|Start%20Game
  ;[1 1 1] Initialize Game
  (CallFunction|SpawnPawns)
  (GameManagement|InitializeGameWidget)
  (EventDispatchers|BindEventtoDiceAnimationEnded (Variables|UI|GetDiceWidget) (delegate Custom|OnDiceAnimationEnded)))

(event Custom|OnDiceAnimationEnded
  ;[1 1 1] Execute Movement
  (Board|MovePawn (Variables|Default|GetCurrentCellDestination))
  (GameManagement|NextTurn))

(event EventBeginPlay
  ;[1 1 1] Wait for all references
  (Utilities|FlowControl|Delay 0.2)
  ;[1 1 1] Camera
  (Game|Player|SetViewTargetwithBlend (Game|GetPlayerController 0) (Variables|GameManagement|GetCameraRef) 0.0 "VTBlend_Linear" 0.0 false)
  ;[1 1 1] Game Instance
  (bind _asbp_game_instance (Utilities|Casting|CastToBP_GameInstance (Game|GetGameInstance)))
  (Variables|GameManagement|SetGIRef _asbp_game_instance)
  ;[1 1 1] Initialize Game
  (Game|SpawnActorfromClass "/Game/Blueprints/BP_PawnController.BP_PawnController_C" (Math|Transform|MakeTransform "0, 0, 0" "0, 0, 0" "1.000000,1.000000,1.000000") "Undefined" "MultiplyWithRoot" 0 0)
  (GameManagement|CreateandAddWidget "/Game/Blueprints/Widgets/WB_Menu.WB_Menu_C")
  (bind _returnvalue (Game|SpawnActorfromClass "/Game/Blueprints/BP_Dice.BP_Dice_C" (Math|Transform|MakeTransform "0, 0, 0" "0, 0, 0" "1.000000,1.000000,1.000000") "Undefined" "MultiplyWithRoot" 0 0))
  (Variables|GameManagement|SetDice _returnvalue))

(fn ConstructionScript)

(fn RollDiceandMove
  (Default|SetButtonState (Variables|UI|GetDiceWidget) false)
  (bind _returnvalue (Class|Dice|Roll (Variables|GameManagement|GetDice) 1))
  (bind _output_get (Variables|Default|SetCurrentCellDestination _returnvalue))
  (Default|BeginDisplayResult (Variables|UI|GetDiceWidget) _output_get))

(fn CreateandAddWidget
  (params (WidgetClass :type User%20Widget%20Class%20Reference))
  (bind _returnvalue (UserInterface|CreateWidget WidgetClass))
  (UserInterface|Viewport|AddtoViewport _returnvalue 0)
  (return _returnvalue))

(fn GetCell
  (params (Index :type Integer))
  (return (Utilities|Array|Get(acopy) (Variables|/Script/BoardGame.Board|GetGrid (Variables|GameManagement|GetBoard)) Index)))

(fn NextTurn
  (if (not (Variables|Default|GetGameIsEnded))
    (if (== (Variables|Player|GetCurrentPlayerTurn) (Variables|Player|GetPlayersNumber))
      (Variables|Player|SetCurrentPlayerTurn 1)
      (else
        (Math|Integer|IncrementInt (Variables|Player|GetCurrentPlayerTurn)
          (:%20%20
            _))))
    (Default|SetButtonState (Variables|UI|GetDiceWidget) true)
    (GameManagement|ModifyText (Utilities|Text|ToText(String) (Utilities|String|Append "It's Player " (Utilities|String|ToString(Integer) (Variables|Player|GetCurrentPlayerTurn)) "'s turn !")))
    (else
      (return))))

(fn GetCurrentPawn
  (return (Utilities|Array|Get(acopy) (Variables|Player|GetPawnsList) (GameManagement|GetCurrentPlayerTurnIndex))))

(fn CheckCellAvailability
  (params (Cell :type Integer))
  (bind _index (Utilities|FlowControl|ForLoopwithBreak 0 (- (Variables|Player|GetPlayersNumber) 1))
    (:LoopBody
      (if (== (.position (Utilities|Array|Get(acopy) (Variables|/Game/Blueprints/BP_GameInstance.BP_GameInstance_C|GetPlayers (Variables|GameManagement|GetGIRef)) _index)) Cell)
        (bind _result (Math|Integer|IncrementInt Cell)
          (:%20%20
            (bind _newcell (Board|CheckCellAvailability _result))
            (return _newcell)))))
    (:Completed
      (return Cell))))

(fn ModifyText
  (params (Text :type Text))
  (Variables|/Script/UMG.TextBlock|SetText (Variables|/Game/Blueprints/Widgets/WB_Dice.WB_Dice_C|GetCurrentPlayerturn (Variables|UI|GetDiceWidget)) Text))

(fn InitializeGameWidget
  (bind _widget (GameManagement|CreateandAddWidget "/Game/Blueprints/Widgets/WB_Dice.WB_Dice_C"))
  (bind _aswb_dice (Utilities|Casting|CastToWB_Dice _widget))
  (bind _output_get (Variables|UI|SetDiceWidget _aswb_dice))
  (Default|SetButtonState _output_get true)
  (GameManagement|ModifyText (Utilities|Text|ToText(String) (Utilities|String|Append "It's Player " (Utilities|String|ToString(Integer) (Variables|Player|GetCurrentPlayerTurn)) "'s turn !"))))

(fn MovePawn
  (params (Increment :type Integer))
  (bind _pawn (Board|GetCurrentPawn))
  (bind _giref (Variables|GameManagement|GetGIRef))
  (bind _players (Variables|/Game/Blueprints/BP_GameInstance.BP_GameInstance_C|GetPlayers _giref))
  (bind _output_get (LocalVariables|SetCurrentPlayerTurnIndex (GameManagement|GetCurrentPlayerTurnIndex)))
  (bind _cell (Default|GetPlayerCellbyID (Variables|GameManagement|GetGIRef) _output_get))
  (bind _newcell (Board|CheckCellAvailability (+ _cell Increment)))
  (LocalVariables|SetCurrentCellIndex (Class|Board|MovePawntoCellbyIndex (Variables|GameManagement|GetBoard) _pawn _newcell))
  (bind _cell_2 (Board|GetCell (LocalVariables|GetCurrentCellIndex)))
  (LocalVariables|SetCurrrentCell _cell_2)
  (Board|RotatePawntoCell _pawn (LocalVariables|GetCurrrentCell))
  (Utilities|Array|SetArrayElem _players (LocalVariables|GetCurrentPlayerTurnIndex) (Utilities|Struct|MakeStruct_Player (.playernumber (Utilities|Array|Get(acopy) _players (LocalVariables|GetCurrentPlayerTurnIndex))) (.score (Utilities|Array|Get(acopy) _players (LocalVariables|GetCurrentPlayerTurnIndex))) (LocalVariables|GetCurrentCellIndex)))
  (Class|Cell|ApplyEffect (LocalVariables|GetCurrrentCell))
  (return (LocalVariables|GetCurrentCellIndex)))

(fn GetCurrentPlayerTurnIndex
  (return (- (Variables|Player|GetCurrentPlayerTurn) 1)))

(fn RotatePawntoCell
  (params (Pawn :type Board%20Pawn%20Object%20Reference) (Cell :type Cell%20Object%20Reference))
  (Transformation|SetActorRotation Pawn (Variables|/Script/BoardGame.Cell|Getrotator Cell)))

(fn AddScore
  (params (Increment :type Integer) (Player%20ID :type Integer))
  (bind _giref (Variables|GameManagement|GetGIRef))
  (bind _players (Variables|/Game/Blueprints/BP_GameInstance.BP_GameInstance_C|GetPlayers _giref))
  (bind _output (Utilities|Array|Get(acopy) _players Player%20ID))
  (Utilities|Array|SetArrayElem _players Player%20ID (Utilities|Struct|MakeStruct_Player (.playernumber _output) (+ Increment (.score _output)) (.position _output))))

(fn GetScore
  (params (PlayerID :type Integer))
  (return (.score (Utilities|Array|Get(acopy) (Variables|/Game/Blueprints/BP_GameInstance.BP_GameInstance_C|GetPlayers (Variables|GameManagement|GetGIRef)) PlayerID))))
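; BP_Cell is a cell actor that sets up its mesh, color and facing.
; The construction script stores the Cylinder as Mesh, passes the white color from DefineColor to ChangeColor, and saves the Arrow component's world rotation as Rotator.
; A separate ReferenceGameMode function casts the current game mode to BP_GameMode and caches it in GMRef.
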(fn ConstructionScript
  (Variables|Default|Setmesh (Variables|Default|GetCylinder))
  (bind _col (CallFunction|DefineColor))
  (Class|Cell|ChangeColor _col)
  (Variables|Default|Setrotator (Transformation|GetWorldRotation (Variables|Default|GetArrow))))

(fn DefineColor
  (return "(R=1.000000,G=1.000000,B=1.000000,A=1.000000)"))

(fn ReferenceGameMode
  (bind _asbp_game_mode (Utilities|Casting|CastToBP_GameMode (Game|GetGameMode)))
  (Variables|Default|SetGMRef _asbp_game_mode))
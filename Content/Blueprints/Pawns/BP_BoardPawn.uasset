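; BP_BoardPawn is a board pawn built from head, body and hand meshes, with a simple procedural idle animation.
; On BeginPlay it gathers the four meshes into an array intended for color changes.
; IdleAnimation re-calls itself after a short delay while State holds one specific value, stepping both hands along relative Z.
; AddAnimationOffset applies each speed-scaled step, and the left hand's limit check flips the shared direction.
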(event Custom|IdleAnimation
  (if (Utilities|Enum|Equal(Enum) (Variables|Animation|GetState) "NewEnumerator0")
    (CallFunction|AddAnimationOffset (Variables|Default|GetRightHand) (Variables|Animation|GetZHandsMax) (Variables|Animation|GetZHandsMin))
    (bind _mustinvertdirection (CallFunction|AddAnimationOffset (Variables|Default|GetLeftHand) (Variables|Animation|GetZHandsMax) (Variables|Animation|GetZHandsMin)))
    (if _mustinvertdirection
      (Variables|Animation|SetDirection (* (Variables|Animation|GetDirection) -1)))
    (Utilities|FlowControl|Delay 0.08)
    (CallFunction|IdleAnimation)))

(event EventBeginPlay
  ;[1 1 1] Reference all meshes that changes color
  (Utilities|Array|AddUnique (Variables|Default|Getmeshes) (Variables|Default|GetHead))
  (Utilities|Array|AddUnique (Variables|Default|Getmeshes) (Variables|Default|GetRightHand))
  (Utilities|Array|AddUnique (Variables|Default|Getmeshes) (Variables|Default|GetLeftHand))
  (Utilities|Array|AddUnique (Variables|Default|Getmeshes) (Variables|Default|GetBody)))

(fn ConstructionScript)

(fn AddAnimationOffset
  (params (Obj :type Static%20Mesh%20Component%20Object%20Reference) (MaxLimit :type Float%20%28double-precision%29) (MinLimit :type Float%20%28double-precision%29))
  (LocalVariables|SetMax MaxLimit)
  (LocalVariables|SetMin MinLimit)
  (LocalVariables|SetO Obj)
  (LocalVariables|SetNewPos (+ (.z (Variables|/Script/Engine.SceneComponent|GetRelativeLocation (LocalVariables|GetO))) (* (Variables|Animation|GetDirection) (* (Variables|Animation|GetIncrement) (Variables|Animation|GetSpeedModifier)))))
  (Transformation|SetRelativeLocation (LocalVariables|GetO) (Math|Vector|MakeVector (.x (Variables|/Script/Engine.SceneComponent|GetRelativeLocation (LocalVariables|GetO))) (.y (Variables|/Script/Engine.SceneComponent|GetRelativeLocation (LocalVariables|GetO))) (LocalVariables|GetNewPos)) false false)
  (return (or (<= (LocalVariables|GetNewPos) (LocalVariables|GetMin)) (>= (LocalVariables|GetNewPos) (LocalVariables|GetMax)))))